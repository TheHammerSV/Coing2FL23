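; Guard AI pawn that investigates camera alerts, patrols that camera's patrol points, then returns to its starting station.
; AI Perception starts a looping chase of visible players, which ends when sight is lost or the player turns invisible.
; A proximity loop or sphere overlap during a chase calls Caught on the player.
; The overlap catch also clears every guard's state and teleports them to their stations after a delay.
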(event `self.ReceiveBeginPlay`
  (set `self.startlocal` (`self.K2_GetActorLocation`))
  (if (and (< (`KismetMathLibrary.Vector_Distance` (`self.K2_GetActorLocation` (`GameplayStatics.GetPlayerCharacter` 0)) (`self.K2_GetActorLocation`)) 200.0) (`self.Chasing`)) :!label _label
    (bind _asbp_first_person_character (cast `/Game/FirstPerson/Blueprints/BP_FirstPersonCharacter` (`GameplayStatics.GetPlayerCharacter` 0)))
    (`/Game/FirstPerson/Blueprints/BP_FirstPersonCharacter.Caught` _asbp_first_person_character)
    (set `self.Chasing` false)
    (`self.ReturnToGuardStation`))
  (`KismetSystemLibrary.Delay` 0.2)
  (goto _label))

(event `Investigate`
  (params (Destination :type "Vector Structure") (Cam :type "/Game/Blueprints/BP_Camera Object Reference"))
  (set `self.PatrolPoints` (`/Game/Blueprints/BP_Camera.PatrolPoints` Cam))
  (`|AIMoveTo` self Destination null 40.0
    (:`OnSuccess`
      (`KismetSystemLibrary.Delay` 1.5))
    (:`OnFail`
      (`KismetSystemLibrary.Delay` 0.1)))
  (`self.Patrol`))

(event `Patrol`
  (set `self.Index` 0)
  (set `self.Patrolling` true)
  (`|AIMoveTo` self (`self.K2_GetActorLocation` (`|GetArrayItem` (`self.PatrolPoints`) (`self.Index`))) null 100.0 :!label _label_2
    (:`OnSuccess`
      (`KismetSystemLibrary.PrintString` "Hello")
      (`KismetSystemLibrary.Delay` 2.0)
      (if (not (`self.Chasing`))
        (`/Engine/EditorBlueprintResources/StandardMacros.IncrementInt` (`self.Index`)
          (:`  `
            (if (>= (`self.Index`) (`KismetArrayLibrary.Array_Length` (`self.PatrolPoints`)))
              (set `self.Patrolling` false)
              (`self.ReturnToGuardStation`)
              (else
                (goto _label_2)))))))))

(event `ReturnToGuardStation`
  (if (not (`self.Chasing`))
    (`|AIMoveTo` self (`self.startlocal`) null 40.0)))

(event `Chase`
  (set `self.Chasing` true)
  (`AIBlueprintHelperLibrary.SimpleMoveToActor` (`self.GetController` self) (`GameplayStatics.GetPlayerCharacter` 0) :!label _label_3)
  (`KismetSystemLibrary.Delay` 0.2)
  (if (`self.Chasing`)
    (goto _label_3)
    (else
      (`self.ReturnToGuardStation`))))

(event `self.PawnSensing.OnSeePawn`
  (params (Pawn :type "Pawn Object Reference")))

(event `self.Sphere.OnComponentBeginOverlap`
  (params (OverlappedComponent :type "PrimitiveComponent Object Reference") (OtherActor :type "Actor Object Reference") (OtherComp :type "PrimitiveComponent Object Reference") (OtherBodyIndex :type Integer) (bFromSweep :type Boolean) (SweepResult :type "HitResult Structure (by ref)"))
  (bind _asbp_first_person_character (cast `/Game/FirstPerson/Blueprints/BP_FirstPersonCharacter` OtherActor))
  (if (`self.Chasing`)
    (`/Game/FirstPerson/Blueprints/BP_FirstPersonCharacter.Caught` _asbp_first_person_character)
    (bind _outactors (`GameplayStatics.GetAllActorsOfClass` "BP_GuardAI_C"))
    (`KismetSystemLibrary.Delay` 2.0)
    (for _array_element _outactors
      (set `/Game/Blueprints/BP_GuardAI.Patrolling` false _array_element)
      (set `/Game/Blueprints/BP_GuardAI.Chasing` false _array_element)
      (`self.ReturnToGuardStation`)
      (`self.K2_SetActorLocation` _array_element (`/Game/Blueprints/BP_GuardAI.startlocal` _array_element) false true))))

(event `self.AIPerception.OnTargetPerceptionUpdated`
  (params (Actor :type "Actor Object Reference") (Stimulus :type "AIStimulus Structure"))
  (bind _asbp_first_person_character (cast `/Game/FirstPerson/Blueprints/BP_FirstPersonCharacter` Actor))
  (if (and (== (`/Game/FirstPerson/Blueprints/BP_FirstPersonCharacter.Invisible` _asbp_first_person_character) false) (`.bSuccessfullySensed` (break `AIStimulus` Stimulus)))
    (`KismetSystemLibrary.PrintString` "Player Seen")
    (set `self.Chasing` true)
    (`self.Chase`)
    (else
      (`KismetSystemLibrary.PrintString` "PlayerLost")
      (set `self.Chasing` false))))

(event `self.ReceiveTick`
  (params (DeltaSeconds :type "Float (single-precision)"))
  (bind _asbp_first_person_character (cast `/Game/FirstPerson/Blueprints/BP_FirstPersonCharacter` (`GameplayStatics.GetPlayerCharacter` 0)))
  (if (and (== (`/Game/FirstPerson/Blueprints/BP_FirstPersonCharacter.Invisible` _asbp_first_person_character) true) (== (`self.Chasing`) true))
    (set `self.Chasing` false)
    (`self.ReturnToGuardStation`)))

(fn `UserConstructionScript`)