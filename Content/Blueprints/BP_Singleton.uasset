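; BP_Singleton manages per-level save data and level transitions, with each save slot named after the current level plus a "_Save" suffix.
; LevelLoad loads the existing BP_SaveLevel and disables every coin in its CollectedCoins list, or creates a fresh save object when none exists.
; LevelSave writes the cached CurrentLevelSave to that slot, and LevelTravel calls it before opening the next level by name.
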(event `LevelLoad`
  (bind _returnvalue (`GameplayStatics.GetCurrentLevelName` true))
  (bind _returnvalue_2 (`KismetStringLibrary.Concat_StrStr` _returnvalue "_Save"))
  (bind _returnvalue_3 (`GameplayStatics.DoesSaveGameExist` _returnvalue_2))
  (if _returnvalue_3
    (bind _returnvalue_4 (`GameplayStatics.LoadGameFromSlot` _returnvalue_2))
    (bind _asbp_save_level (cast `/Game/Blueprints/BP_SaveLevel` _returnvalue_4))
    (set `self.CurrentLevelSave` _asbp_save_level)
    (for _array_element (`/Game/Blueprints/BP_SaveLevel.CollectedCoins` _asbp_save_level)
      (`/Game/Blueprints/BP_Collectible.DisableCoin` _array_element))
    (else
      (bind _returnvalue_5 (`GameplayStatics.CreateSaveGameObject` "/Game/Blueprints/BP_SaveLevel.BP_SaveLevel_C"))
      (set `self.CurrentLevelSave` _returnvalue_5))))

(event `LevelSave`
  (bind _returnvalue (`GameplayStatics.GetCurrentLevelName` true))
  (`GameplayStatics.SaveGameToSlot` (`self.CurrentLevelSave`) (`KismetStringLibrary.Concat_StrStr` _returnvalue "_Save")))

(event `LevelTravel`
  (params (NextLevel :type Name))
  (`self.LevelSave`)
  (`GameplayStatics.OpenLevel` NextLevel))