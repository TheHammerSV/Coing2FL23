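; Security camera actor that spots the first-person player with AI perception and dispatches its assigned guards to investigate.
; On a successful sighting it waits a second, then, unless the player is invisible, calls Investigate on each guard with the player's location.
; Tick also sends guards while the player stays visible and sending is allowed, and each dispatch clears that flag.
; Debug prints and boxes mark perception updates.
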(event `self.ReceiveBeginPlay`)

(event `self.AIPerception.OnTargetPerceptionUpdated`
  (params (Actor :type "Actor Object Reference") (Stimulus :type "AIStimulus Structure"))
  (bind (_age _expirationage _strength _stimuluslocation _receiverlocation _tag _bsuccessfullysensed) (break `AIStimulus` Stimulus))
  (bind _asbp_first_person_character (cast `/Game/FirstPerson/Blueprints/BP_FirstPersonCharacter` Actor))
  (set `self.CanSeePlayer` _bsuccessfullysensed)
  (`|ExecutionSequence`
    (:`then_0`
      (if _bsuccessfullysensed
        (`KismetSystemLibrary.PrintString` "I can see the player")
        (`KismetSystemLibrary.Delay` 1.0)
        (set `self.CanSendGuards` true)
        (bind _asbp_first_person_character_2 (cast `/Game/FirstPerson/Blueprints/BP_FirstPersonCharacter` (`GameplayStatics.GetPlayerCharacter` 0)))
        (if (not (`/Game/FirstPerson/Blueprints/BP_FirstPersonCharacter.Invisible` _asbp_first_person_character_2))
          (`self.SendGuards` (`self.K2_GetActorLocation` _asbp_first_person_character)))
        (else
          (`KismetSystemLibrary.PrintString` "I lost the player")
          (set `self.CanSendGuards` false))))
    (:`then_1`
      (`KismetSystemLibrary.DrawDebugBox` _stimuluslocation (0.0 0.0 0.0) (struct) (struct) 30.0 50.0))))

(event `SendGuards`
  (params (PlayerLocation :type "Vector Structure"))
  (set `self.CanSendGuards` false)
  (if (`self.CanSeePlayer`)
    (for _array_element (`self.AssignedGuards`)
      (`KismetSystemLibrary.PrintString` "Hunt")
      (`/Game/Blueprints/BP_GuardAI.Investigate` _array_element PlayerLocation self))))

(event `self.ReceiveTick`
  (params (DeltaSeconds :type "Float (single-precision)"))
  (if (and (== (`self.CanSeePlayer`) true) (== (`self.CanSendGuards`) true) (== (`/Game/FirstPerson/Blueprints/BP_FirstPersonCharacter.Invisible` (cast `/Game/FirstPerson/Blueprints/BP_FirstPersonCharacter` (`GameplayStatics.GetPlayerCharacter` 0) :!pure true)) false))
    (`self.SendGuards` (`self.K2_GetActorLocation` (`GameplayStatics.GetPlayerCharacter` 0)))))

(fn `UserConstructionScript`)