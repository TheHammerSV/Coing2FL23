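; BP_Collectible is a pickup that bobs vertically and adds one to the score when the first-person character touches it.
; A timeline applies scaled local Z offsets to the mesh each update, restarting on finish through a FlipFlop that alternates the direction.
; Overlapping the collision component increments Score on the BP_Singleton game instance and destroys the actor.
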(event `self.ReceiveBeginPlay`
  (bind (_direction _positionoffset) (`Timeline|Animation` :!via `PlayFromStart` :!label _label)
    (:`Update`
      (if (stale _isa)
        (bind _returnvalue (* _positionoffset 0.25))
        (`SceneComponent.K2_AddLocalOffset` (`self.Mesh`) (`KismetMathLibrary.MakeVector` 0.0 0.0 (* _returnvalue -1.0)) false false)
        (else
          (`SceneComponent.K2_AddLocalOffset` (`self.Mesh`) (`KismetMathLibrary.MakeVector` 0.0 0.0 _returnvalue) false false))))
    (:`Finished`
      (bind _isa (`/Engine/EditorBlueprintResources/StandardMacros.FlipFlop`)
        (:`A`
          (goto _label :!via `PlayFromStart`))
        (:`B`
          (goto _label :!via `PlayFromStart`))))))

(event `self.CollectCollision.OnComponentBeginOverlap`
  (params (OverlappedComponent :type "PrimitiveComponent Object Reference") (OtherActor :type "Actor Object Reference") (OtherComp :type "PrimitiveComponent Object Reference") (OtherBodyIndex :type Integer) (bFromSweep :type Boolean) (SweepResult :type "HitResult Structure (by ref)"))
  (cast `/Game/FirstPerson/Blueprints/BP_FirstPersonCharacter` OtherActor)
  (bind _asbp_singleton (cast `/Game/Blueprints/BP_Singleton` (`GameplayStatics.GetGameInstance`)))
  (`/Engine/EditorBlueprintResources/StandardMacros.IncrementInt` (`/Game/Blueprints/BP_Singleton.Score` _asbp_singleton)
    (:`  `
      (`self.K2_DestroyActor`))))

(fn `UserConstructionScript`)