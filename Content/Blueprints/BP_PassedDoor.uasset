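; One-shot trigger that marks the player passing a door between areas, acting as a checkpoint and scoring point.
; On first overlap it saves its location to BP_GameInstance, loads the area's card count and resets the collected tally.
; For BP_FirstPersonCharacter it resets invisibility, awards area points plus a bonus per still-valid guard, and switches the linked door.
; If flagged Final with a valid door, it also shows the end screen with UI-only input.
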(event `self.ReceiveActorBeginOverlap`
  (params (OtherActor :type "Actor Object Reference"))
  (bind _returnvalue (`GameplayStatics.GetPlayerController` 0))
  (bind _door (`self.Door`))
  (`/Engine/EditorBlueprintResources/StandardMacros.DoOnce` false
    (:`Completed`
      (bind _asbp_game_instance (cast `/Game/Blueprints/BP_GameInstance` (`GameplayStatics.GetGameInstance`)))
      (set `/Game/Blueprints/BP_GameInstance.SavedCheckpoint` true _asbp_game_instance)
      (set `/Game/Blueprints/BP_GameInstance.LastCheckpoint` (`self.K2_GetActorLocation`) _asbp_game_instance)
      (bind _asbp_game_instance_2 (cast `/Game/Blueprints/BP_GameInstance` (`GameplayStatics.GetGameInstance`)))
      (set `/Game/Blueprints/BP_GameInstance.NumCards` (`self.NumAreaCards`) _asbp_game_instance_2)
      (set `/Game/Blueprints/BP_GameInstance.NumCardsCollected` 0 _asbp_game_instance_2)
      (bind _asbp_first_person_character (cast `/Game/FirstPerson/Blueprints/BP_FirstPersonCharacter` OtherActor))
      (`/Game/FirstPerson/Blueprints/BP_FirstPersonCharacter.ResetInvisInstant` _asbp_first_person_character)
      (bind _asbp_game_instance_3 (cast `/Game/Blueprints/BP_GameInstance` (`GameplayStatics.GetGameInstance`)))
      (set `/Game/Blueprints/BP_GameInstance.Points` (+ (`/Game/Blueprints/BP_GameInstance.Points` _asbp_game_instance_3) (`self.PointsWorth`)) _asbp_game_instance_3)
      (for _array_element (`self.AreaGuards`)
        (`/Engine/EditorBlueprintResources/StandardMacros.IsValid` _array_element
          (:`Is Valid`
            (set `/Game/Blueprints/BP_GameInstance.Points` (+ (`/Game/Blueprints/BP_GameInstance.Points` _asbp_game_instance_3) 25) _asbp_game_instance_3))))
      (`/Engine/EditorBlueprintResources/StandardMacros.IsValid` _door
        (:`Is Valid`
          (`/Game/Blueprints/BP_Door.SwitchDoor` _door true)
          (if (`self.Final`)
            (bind _returnvalue_2 (`|CreateWidget` "/Game/Blueprints/W_End.W_End_C"))
            (`UserWidget.AddToViewport` _returnvalue_2 0)
            (`WidgetBlueprintLibrary.SetInputMode_UIOnlyEx` _returnvalue null)
            (set `PlayerController.bShowMouseCursor` true _returnvalue)))))))

(fn `UserConstructionScript`)