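; BP_HomeworkAI is a simple patrolling AI pawn that wanders out from its spawn point and returns.
; On BeginPlay it stores its location as Origin, then moves to a random navigable point within a radius of it using AIMoveTo.
; After a short delay it walks back to Origin, waits again and repeats.
; The loop continues only on successful moves, as failures are unhandled.
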(event `self.ReceiveBeginPlay`
  (set `self.Origin` (`self.K2_GetActorLocation`))
  (`self.Patrol`))

(event `Patrol`
  (bind _randomlocation (`NavigationSystemV1.K2_GetRandomLocationInNavigableRadius` (`self.Origin`) 5000.0 null null))
  (`|AIMoveTo` self _randomlocation null
    (:`OnSuccess`
      (`KismetSystemLibrary.Delay` 2.0)
      (`|AIMoveTo` self (`self.Origin`) null
        (:`OnSuccess`
          (`KismetSystemLibrary.Delay` 2.0)
          (`self.Patrol`))))))

(fn `UserConstructionScript`)